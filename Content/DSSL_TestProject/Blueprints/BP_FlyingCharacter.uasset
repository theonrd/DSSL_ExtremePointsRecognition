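; Flying character for a scanning demo that photographs a target skeletal mesh through a full turn, marking its extreme vertices.
; BeginPlay adds the HUD and grabs the first BP_Target's mesh.
; F clears the screenshot folder, then a self-recalling timeline event rotates the mesh in 36 steps.
; After each step, extreme LOD0 vertices are screen-projected via the player controller, drawn onto the scene capture's render target and saved.
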(event Custom|AddRotationAndTakeShot
  (params (Iterations :type Integer))
  (bind _returnvalue (- Iterations 1))
  (Variables|Target|SetSkeletalPreviousPointRotator (Variables|/Script/Engine.SceneComponent|GetRelativeRotation (Variables|Target|GetSkeletalMeshForScan)))
  (bind _rotateadditional (Timeline|Rotate PlayFromStart)
    (:Update
      (Transformation|SetRelativeRotation (Variables|Target|GetSkeletalMeshForScan) (Math|Rotator|Lerp(Rotator) (Variables|Target|GetSkeletalPreviousPointRotator) (Math|Rotator|CombineRotators (Variables|Target|GetSkeletalPreviousPointRotator) "0.000000,10.000000,0.000000") _rotateadditional true) false false))
    (:Finished
      (CallFunction|TakeScreenshotwithExtremePoints (Utilities|String|ToString(Integer) Iterations))
      (if (> _returnvalue 0)
        (CallFunction|AddRotationandTakeShot _returnvalue)))))

(event EventBeginPlay
  (CallFunction|CreateHUD)
  (CallFunction|AssignTargetSkeletalMesh))

(event Input|KeyboardEvents|F
  (params (Key :type Key%20Structure))
  (:Pressed
    (Utilities|IsValid (Variables|Target|GetSkeletalMeshForScan)
      (:Is%20Valid
        (Class|ScreenshotTools|DeleteDirectory (Variables|Screenshot|GetScreenShotsRelativeFolder))
        (CallFunction|AddRotationandTakeShot 36)))))

(fn ConstructionScript)

(fn TakeScreenshotwithExtremePoints
  (params (FileName :type String))
  (bind _scenecapturecomponent2d (Variables|Default|GetSceneCaptureComponent2D))
  (bind _texturetarget (Variables|/Script/Engine.SceneCaptureComponent2D|GetTextureTarget _scenecapturecomponent2d))
  (bind _outvertices (Class|ExtremePointsRecognition|GetSkeletalMeshVertices (Variables|Target|GetSkeletalMeshForScan)))
  (bind _returnvalue (Class|ExtremePointsRecognition|ProjectExtremeVerticestoScreen (Game|GetPlayerController 0) _outvertices))
  (Class|ScreenshotTools|OverlayPointstoRenderTarget _texturetarget _returnvalue (Variables|RenderedPoints|GetPointSize) (Variables|RenderedPoints|GetPointTexture) (Variables|RenderedPoints|GetPointColor))
  (Class|ScreenshotTools|TakeRenderTargetShot _texturetarget (Variables|Screenshot|GetScreenShotsRelativeFolder) FileName))

(fn AssignTargetSkeletalMesh
  ;[1 1 1] It's for demonstration purposes only :)
  (bind _outactors (Actor|GetAllActorsOfClass "/Game/DSSL_TestProject/Blueprints/BP_Target.BP_Target_C"))
  (Variables|Target|SetSkeletalMeshForScan (Variables|/Game/DSSL_TestProject/Blueprints/BP_Target.BP_Target_C|GetSkeletalMesh (Utilities|Array|Get(acopy) _outactors))))

(fn CreateHUD
  (bind _returnvalue (UserInterface|CreateWidget "/Game/DSSL_TestProject/Blueprints/W_IngameHUD.W_IngameHUD_C"))
  (UserInterface|Viewport|AddtoViewport _returnvalue 0))